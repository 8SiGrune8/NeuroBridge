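; BP_OSCTestReceiver is a test actor that receives OSC messages and scales a Sphere by the received value.
; On BeginPlay it creates a listening OSC server on localhost port 7001 and binds a message handler.
; The handler stores each message's first float as MindState, prints it and sets it as the Sphere's uniform world scale, without address filtering or clamping.
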(event `self.ReceiveBeginPlay`
  (bind _returnvalue (`OSCManager.CreateOSCServer` "127.0.0.1" 7001 false true "TestServer" self))
  (add `OSCServer.OnOscMessageReceived` _returnvalue (delegate `OSC_Message_Received`)))

(event `OSC_Message_Received`
  (params (Message :type "OSCMessage Structure (by ref)") (IPAddress :type String) (Port :type Integer))
  (bind _mindstate (`self.MindState`))
  (bind _value (`OSCManager.GetFloat` Message))
  (set `self.MindState` _value)
  (`KismetSystemLibrary.PrintString` (`KismetStringLibrary.Conv_DoubleToString` (`self.MindState`)) true true (struct :`G` 0.66 :`B` 1.0 :`A` 1.0) 20.0)
  (`SceneComponent.SetWorldScale3D` (`self.Sphere`) (`KismetMathLibrary.MakeVector` _mindstate _mindstate _mindstate)))

(fn `UserConstructionScript`)