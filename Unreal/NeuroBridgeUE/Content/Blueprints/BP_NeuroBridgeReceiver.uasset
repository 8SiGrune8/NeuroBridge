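; BP_NeuroBridgeReceiver is a work-in-progress OSC receiver that currently only prints debug output.
; On BeginPlay it starts an OSC server listening on localhost port 7001, prints diagnostics and binds a message-received handler.
; That handler prints a receipt notice and the sender IP, without reading the message.
; Disconnected nodes sketch unfinished `/neuro/mindstate` address matching, MindState float extraction and an OSC client.
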(event `OSC_Message_Received_Pattern`
  (params (AddressPattern :type "OSCAddress Structure (by ref)") (Message :type "OSCMessage Structure (by ref)") (IPAddress :type String) (Port :type Integer)))

(event `self.ReceiveBeginPlay`
  (bind _returnvalue (`OSCManager.CreateOSCServer` "127.0.0.1" 7001 false true "" self))
  (set `self.OSC_Server` _returnvalue)
  (`KismetSystemLibrary.PrintString` (`KismetStringLibrary.Conv_IntToString` (`KismetArrayLibrary.Array_Length` (`OSCServer.GetBoundOSCAddressPatterns` (`self.OSC_Server`)))) true true (struct :`G` 0.66 :`B` 1.0 :`A` 1.0) 20.0)
  (`KismetSystemLibrary.PrintString` (`KismetSystemLibrary.GetDisplayName` (`self.OSC_Server`)) true true (struct :`G` 0.66 :`B` 1.0 :`A` 1.0) 25.0)
  (bind _output_get (set `self.OSC_Address` (make `OSCAddress`)))
  (bind _returnvalue_2 (`OSCManager.GetOSCAddressFullPath` _output_get))
  (`KismetSystemLibrary.PrintString` _returnvalue_2 true true (struct :`G` 0.66 :`B` 1.0 :`A` 1.0) 20.0)
  (add `OSCServer.OnOscMessageReceived` (`self.OSC_Server`) (delegate `OSC_Message_Received`)))

(event `OSC_Message_Received`
  (params (Message :type "OSCMessage Structure (by ref)") (IPAddress :type String) (Port :type Integer))
  (`KismetSystemLibrary.PrintString` "OSC Received" true true (struct :`G` 0.66 :`B` 1.0 :`A` 1.0) 25.0)
  (`KismetSystemLibrary.PrintString` IPAddress true true (struct :`G` 0.66 :`B` 1.0 :`A` 1.0) 20.0))

(event `OnOSCMessageReceivedEvent`
  (`KismetSystemLibrary.PrintString` "OSC Received" true true (struct :`G` 0.66 :`B` 1.0 :`A` 1.0) 30.0))

(fn `UserConstructionScript`)